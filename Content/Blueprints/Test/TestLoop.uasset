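; TestLoop is a test Blueprint that exercises array iteration on BeginPlay.
; It fills the Ages array with a few integers, sums them into Sum with a for-each loop, and prints the total to screen.
; The overlap, Tick and construction script graphs are empty.
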(event EventBeginPlay
  (bind _ages (Variables|Default|GetAges))
  (Utilities|Array|Add _ages 22)
  (Utilities|Array|Add _ages 23)
  (Utilities|Array|Add _ages 24)
  (for _array_element _ages
    (Variables|Default|SetSum (+ _array_element (Variables|Default|GetSum))))
  (Development|PrintString (Utilities|String|ToString(Integer) (Variables|Default|GetSum))))

(event Collision|EventActorBeginOverlap
  (params (OtherActor :type Actor%20Object%20Reference)))

(event EventTick
  (params (DeltaSeconds :type Float%20%28single-precision%29)))

(fn ConstructionScript)