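; Game instance that manages persistent save data: one global save plus a separate save per listed player.
; On Init it loads the GlobalData slot, or creates a new save object if loading fails.
; After a successful load, each PlayerList entry serves as a slot name to fill PlayerDataArray with PlayerData saves.
; AddPlater registers names without duplicates, and SaveOll writes only the global object back to disk.
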(event EventInit
  ;[1 1 1] 初始化事件   发生在非常早的时候
  (Utilities|FlowControl|Sequence
    (:then_0
      (bind _returnvalue (SaveGame|LoadGamefromSlot "GlobalDada"))
      (bind _asglobal_data (Utilities|Casting|CastToGlobalData _returnvalue)
        (:then
          (Variables|Default|SetGlobalDada _asglobal_data)
          (CallFunction|InitPlayerData))
        (:CastFailed
          (bind _returnvalue_2 (SaveGame|CreateSaveGameObject "/Game/Blueprints/GlobalData.GlobalData_C"))
          (Variables|Default|SetGlobalDada _returnvalue_2))))))

(fn InitPlayerData
  (for (_ _array_index) (Variables|/Game/Blueprints/GlobalData.GlobalData_C|GetPlayerList (Variables|Default|GetGlobalDada))
    (bind _returnvalue (SaveGame|LoadGamefromSlot (Utilities|String|ToString(Integer) _array_index)))
    (Utilities|Casting|CastToPlayerData _returnvalue)
    (Utilities|Array|Add (Variables|Default|GetPlayerDataArray) 0)))

(fn AddPlater
  (params (Name :type Text))
  ;[1 1 1] 数组有重复就不添加了
  (Utilities|Array|AddUnique (Variables|/Game/Blueprints/GlobalData.GlobalData_C|GetPlayerList (Variables|Default|GetGlobalDada)) Name))

(fn SaveOll
  (SaveGame|SaveGametoSlot (Variables|Default|GetGlobalDada) "GlobalDada"))